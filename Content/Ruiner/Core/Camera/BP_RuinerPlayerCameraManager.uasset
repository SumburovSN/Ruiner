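; Player camera manager for Ruiner that orbits the view target and always looks at it, with a fixed field of view.
; BlueprintUpdateCamera places the camera on a sphere from surface angle, radial angle and distance using trigonometry, overriding the default camera.
; Radial rotation requests shift a target angle that Tick smoothly interpolates toward, while events step the zoom distance.
; Helper events enable or disable camera modifiers by class, adding missing ones on demand.
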(event Custom|ReduceDistance
  (Variables|Default|SetDistanceToCamera (- (Variables|Default|GetDistanceToCamera) 2e+01)))

(event Custom|IncreaseDistance
  (Variables|Default|SetDistanceToCamera (+ (Variables|Default|GetDistanceToCamera) 2e+01)))

(event Custom|EnableCameraModifier
  (params (ModifierClass :type Camera%20Modifier%20Class%20Reference))
  (bind _returnvalue (Game|Player|FindCameraModifierbyClass ModifierClass))
  (Utilities|IsValid _returnvalue
    (:Is%20Valid
      (CameraModifier|EnableModifier _returnvalue))
    (:Is%20Not%20Valid
      (Game|Player|AddNewCameraModifier ModifierClass))))

(event Custom|DisableCameraModifier
  (params (ModifierClass :type Camera%20Modifier%20Class%20Reference) (Immediate :type Boolean))
  (bind _returnvalue (Game|Player|FindCameraModifierbyClass ModifierClass))
  (Utilities|IsValid _returnvalue
    (:Is%20Valid
      (CameraModifier|DisableModifier _returnvalue Immediate))))

(event EventBeginPlay
  (bind _output_get (Variables|Default|SetRuinerPlayerController (.AsBP%20Ruiner%20Player%20Controller (Utilities|Casting|CastToBP_RuinerPlayerController (Game|Player|GetOwningPlayerController)))))
  (Game|Player|SetViewTargetwithBlend _output_get _output_get 0.0 "VTBlend_Linear" 0.0 false))

(event EventTick
  (params (DeltaSeconds :type Float%20%28single-precision%29))
  (Utilities|InterpRadialAngle))

(fn ConstructionScript)

(fn BlueprintUpdateCamera
  (params (CameraTarget :type Actor%20Object%20Reference))
  (bind _returnvalue (Transformation|GetActorLocation CameraTarget))
  (bind _surfaceangle (Variables|Default|GetSurfaceAngle))
  (bind _distancetocamera (Variables|Default|GetDistanceToCamera))
  (bind _surfaceangle_2 (Variables|Default|GetSurfaceAngle))
  (bind _distancetocamera_2 (Variables|Default|GetDistanceToCamera))
  (bind _currentradialangle (Variables|Default|GetCurrentRadialAngle))
  (bind _returnvalue_2 (Math|Trig|Sin(Degrees) _surfaceangle_2))
  (bind _returnvalue_3 (Math|Trig|Cos(Degrees) _surfaceangle))
  (bind _returnvalue_4 (Math|Trig|Sin(Degrees) _currentradialangle))
  (bind _returnvalue_5 (Math|Trig|Cos(Degrees) _currentradialangle))
  (bind _returnvalue_6 (* _returnvalue_3 _distancetocamera))
  (bind _returnvalue_7 (* _returnvalue_2 _distancetocamera_2))
  (bind _returnvalue_8 (* _returnvalue_6 _returnvalue_5))
  (bind _returnvalue_9 (* _returnvalue_6 _returnvalue_4))
  (bind _returnvalue_10 (+ _returnvalue (Math|Vector|MakeVector _returnvalue_9 _returnvalue_8 _returnvalue_7)))
  (return _returnvalue_10 (Math|Rotator|FindLookatRotation _returnvalue_10 _returnvalue) 9e+01 true))

(fn IncreaseRadialAngle
  (params (DeltaAngle :type Float%20%28single-precision%29))
  (Variables|Default|SetTargetRadialAngle (+ DeltaAngle (Variables|Default|GetTargetRadialAngle))))