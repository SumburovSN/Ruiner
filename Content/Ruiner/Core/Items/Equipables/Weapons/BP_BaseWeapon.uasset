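; Base weapon Blueprint that provides the shared fire and reload flow, with stub functions for ammo checks, ammo use and play rate.
; Fire checks readiness, ammo and loaded state, then either fires, reloads or calls the empty NoAmmo event.
; The fire montage's completion or interruption restores readiness, so its play rate sets fire cadence.
; Reload broadcasts OnReload and restores readiness after a retriggerable delay.
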(event Custom|NoAmmo)

(event Custom|Fire
  (if (Variables|Default|GetbRdyToFire)
    (bind _bammunition (CallFunction|CheckAmmunition))
    (if _bammunition
      (bind _bloaded (CallFunction|CheckLoaded))
      (if _bloaded
        (Components|Animation|SetAnimation (Variables|Default|GetSkeletalMesh) (Variables|Default|GetW_Fire))
        (Variables|Default|SetbRdyToFire false)
        (CallFunction|UseAmmunition)
        (Variables|Default|SetbReloaded false)
        (CallFunction|OnReadytoFire)
        (else
          (CallFunction|Reload)))
      (else
        (CallFunction|NoAmmo)))))

(event Custom|OnReadyToFire
  (Animation|Montage|PlayMontage (Variables|Default|GetSkeletalMesh) (Variables|Default|GetW_Fire) (CallFunction|GetFireAnimationPlayRate)
    (:OnCompleted
      _)
    (:OnInterrupted
      _))
  (Variables|Default|SetbRdyToFire true))

(event Custom|OnFired)

(event Custom|Reload
  (bind _reloadtime (Variables|Default|GetReloadTime))
  (Variables|Default|SetbReloadInProgress true)
  (Variables|Default|SetbRdyToFire false)
  (Default|CallOnReload _reloadtime)
  (Utilities|FlowControl|RetriggerableDelay _reloadtime)
  (Variables|Default|SetbRdyToFire true)
  (Variables|Default|SetbReloadInProgress false)
  (Variables|Default|SetbReloaded true))

(event EventBeginPlay)

(fn ConstructionScript)

(fn CheckAmmunition
  (return true))

(fn CheckLoaded
  (return true))

(fn UseAmmunition)

(fn GetFireAnimationPlayRate
  (return 1.0))