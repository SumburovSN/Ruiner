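; Projectile weapon Blueprint in the ammo weapon family that launches a projectile actor each time it fires.
; OnFired runs the parent logic, then spawns ProjectileClass at the skeletal mesh's Muzzle socket, ignoring collisions.
; The shot takes the owner actor's rotation instead of the socket's, with the weapon as Owner and the owning pawn as Instigator.
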(event EventOnFired
  (|CallParentFunction)
  (Game|SpawnActorfromClass (Variables|Default|GetProjectileClass) (Math|Transform|MakeTransform (Transformation|GetSocketLocation (Variables|Default|GetSkeletalMesh) "Muzzle") (Transformation|GetActorRotation (Components|GetOwner)) "1,1,1") "AlwaysSpawn" self (.AsPawn (Utilities|Casting|CastToPawn (Components|GetOwner)))))

(fn ConstructionScript
  (|CallParentFunction))