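; Base weapon projectile that branches its impact behavior on a remaining split depth.
; On hit with depth left, it calls OnSplit, then immediately spawns its explosion effect and destroys itself.
; At zero depth or below, it waits for a hit destroy delay, calls OnSplitEnd, then explodes and destroys itself.
; Both split functions are empty hooks here, so this asset spawns no child projectiles itself.
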(event EventOnHit
  (if (<= (Variables|Default|GetSplitDepth) 0)
    (Utilities|FlowControl|Delay (Variables|Default|GetHitDestroyDelay))
    (CallFunction|OnSplitEnd)
    (CallFunction|SpawnExplosionEffectandDestroy)
    (else
      (CallFunction|OnSplit)
      (CallFunction|SpawnExplosionEffectandDestroy))))

(fn ConstructionScript
  (|CallParentFunction))

(fn OnSplit
  (return))

(fn OnSplitEnd)