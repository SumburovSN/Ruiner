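; Base projectile actor for projectile weapons that deals damage through a spawned actor and plays flight, bounce and explosion effects.
; On BeginPlay it async-loads its sounds and particle system in parallel, attaching the in-air loop to the Box.
; Box hits, ignoring owner and instigator, trigger a delayed damage-actor spawn and explosion.
; The projectile destroys itself only when both explosion particle and sound are loaded.
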(event OnComponentHit(Box)
  (params (HitComponent :type Primitive%20Component%20Object%20Reference) (OtherActor :type Actor%20Object%20Reference) (OtherComp :type Primitive%20Component%20Object%20Reference) (NormalImpulse :type Vector :default "0, 0, 0") (Hit :type Hit%20Result%20Structure%20%28by%20ref%29))
  (if (and (!= OtherActor (Components|GetOwner)) (!= OtherActor (Game|GetInstigator)))
    (CallFunction|OnHit)))

(event OnProjectileBounce(ProjectileMovement)
  (params (ImpactResult :type Hit%20Result%20Structure%20%28by%20ref%29) (ImpactVelocity :type Vector%20%28by%20ref%29 :default "0, 0, 0"))
  (bind _bouncecueloaded (Variables|Default|GetBounceCueLoaded))
  (Utilities|IsValid _bouncecueloaded
    (:Is%20Valid
      (Audio|PlaySoundatLocation _bouncecueloaded (Transformation|GetActorLocation) "0, 0, 0" 1.0 1.0 0.0 0 0 0))))

(event Custom|SpawnExplosionEffectAndDestroy
  (bind _returnvalue (Transformation|GetActorLocation))
  (bind _destroypsloaded (Variables|Default|GetDestroyPSLoaded))
  (bind _explosioncueloaded (Variables|Default|GetExplosionCueLoaded))
  (Utilities|IsValid _destroypsloaded
    (:Is%20Valid
      (Effects|SpawnEmitteratLocation _destroypsloaded _returnvalue)
      (Utilities|IsValid _explosioncueloaded
        (:Is%20Valid
          (Audio|PlaySoundatLocation _explosioncueloaded _returnvalue "0, 0, 0" 1.0 1.0 0.0 0 0 0)
          (Actor|DestroyActor))))))

(event Custom|OnHit
  (Utilities|FlowControl|Delay (Variables|Default|GetHitDestroyDelay))
  (Game|SpawnActorfromClass (Variables|Default|GetDamageActorClass) (Math|Transform|MakeTransform (Transformation|GetActorLocation) "0, 0, 0" "1,1,1") "Undefined" (Components|GetOwner) 0)
  (CallFunction|SpawnExplosionEffectandDestroy))

(event EventBeginPlay
  (bind _object (Utilities|AsyncLoadAsset (Variables|Default|GetInAirLoop))
    (:then
      (bind _object_2 (Utilities|AsyncLoadAsset (Variables|Default|GetExplosionCue))
        (:then
          (bind _object_3 (Utilities|AsyncLoadAsset (Variables|Default|GetDestroy_PS))
            (:then
              (bind _object_4 (Utilities|AsyncLoadAsset (Variables|Default|GetBounceCue))
                (:Completed
                  (Variables|Default|SetBounceCueLoaded (.AsSound%20Cue (Utilities|Casting|CastToSoundCue _object_4))))))
            (:Completed
              (Variables|Default|SetDestroyPSLoaded (.AsParticle%20System (Utilities|Casting|CastToParticleSystem _object_3))))))
        (:Completed
          (Variables|Default|SetExplosionCueLoaded (.AsSound%20Cue (Utilities|Casting|CastToSoundCue _object_2))))))
    (:Completed
      (Audio|SpawnSoundAttached (.AsSound%20Cue (Utilities|Casting|CastToSoundCue _object)) (Variables|Default|GetBox) "None" "0, 0, 0" "0, 0, 0" "KeepRelativeOffset" false 1.0 1.0 0.0 0 0))))

(fn ConstructionScript)