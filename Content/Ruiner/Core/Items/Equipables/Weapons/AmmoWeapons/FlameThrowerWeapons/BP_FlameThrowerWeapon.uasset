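; Flamethrower ammo weapon that sprays a continuous flame while fire input keeps arriving.
; Each Fire call refreshes a retriggerable delay that ends firing on timeout, and the first also async-loads and attaches the flame particles.
; While firing, Tick uses ammo and spawns damage actors from the flame socket at a fixed rate, stopping when empty.
; Stopping detaches the particles and disables their emitters; unequipping is blocked while firing.
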(event Custom|StartFiring
  (if (Variables|Default|GetbFiring)
    (Utilities|FlowControl|RetriggerableDelay (Variables|Default|GetFireEndTime) :!label _label)
    (CallFunction|EndFiring)
    (else
      (CallFunction|CheckAmmunition)
      (if true
        (Variables|Default|SetbFiring true)
        (bind _object (Utilities|AsyncLoadAsset (Variables|Default|GetFlamePS))
          (:then
            (goto _label))
          (:Completed
            (bind _returnvalue (Effects|SpawnEmitterAttached (.AsParticle%20System (Utilities|Casting|CastToParticleSystem _object)) (Variables|Default|GetSkeletalMesh) (Variables|Default|GetFlameSocket)))
            (Variables|Default|SetFlamePSComponent _returnvalue)))
        (else
          (CallFunction|NoAmmo))))))

(event Custom|EndFiring
  (Variables|Default|SetbFiring false)
  (Variables|Default|SetTickShotsTimer 0.0)
  (Utilities|IsValid (Variables|Default|GetFlamePSComponent)
    (:Is%20Valid
      (Transformation|DetachFromComponent (Variables|Default|GetFlamePSComponent) "KeepRelative" "KeepRelative" "KeepRelative" true)
      (Effects|Components|ParticleSystem|SetEmitterEnable (Variables|Default|GetFlamePSComponent) "Emitter0" false)
      (Effects|Components|ParticleSystem|SetEmitterEnable (Variables|Default|GetFlamePSComponent) "Emitter1" false)
      (Variables|Default|SetFlamePSComponent 0))))

(event EventBeginPlay
  (|CallParentFunction) ; This node is disabled and will not be called.\nDrag off pins to build functionality.
)

(event EventTick
  (params (DeltaSeconds :type Float%20%28single-precision%29))
  (bind _skeletalmesh (Variables|Default|GetSkeletalMesh))
  (bind _returnvalue (Transformation|GetWorldRotation _skeletalmesh))
  (if (Variables|Default|GetbFiring)
    (bind _output_get (Variables|Default|SetTickShotsTimer (+ DeltaSeconds (Variables|Default|GetTickShotsTimer))))
    (if (>= _output_get (/ 1.0 (Variables|Default|GetShotsPerSecond)))
      (CallFunction|UseAmmunition)
      (Variables|Default|SetTickShotsTimer 0.0)
      (Game|SpawnActorfromClass (Variables|Default|GetDamageActorClass) (Math|Transform|MakeTransform (Transformation|GetSocketLocation _skeletalmesh (Variables|Default|GetFlameSocket)) (Math|Rotator|MakeRotator (.roll _returnvalue) (- (.pitch _returnvalue) 9e+01) (+ (.yaw _returnvalue) 9e+01)) "1,1,1") "Undefined" self 0)
      (bind _bammunition (CallFunction|CheckAmmunition))
      (if (not _bammunition)
        (CallFunction|NoAmmo)
        (CallFunction|EndFiring)))))

(event EventFire
  (CallFunction|StartFiring))

(fn ConstructionScript
  (|CallParentFunction))

(fn CanUnequipItem
  (return (not (Variables|Default|GetbFiring))))