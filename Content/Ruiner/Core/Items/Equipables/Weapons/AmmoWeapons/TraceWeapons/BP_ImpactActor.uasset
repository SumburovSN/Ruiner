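; BP_ImpactActor is a short-lived effect actor that shows a weapon impact's particles and optional sound for the surface hit.
; SetTag takes the first surface tag found in SurfaceMap, picks that entry's particle system by impact size, and async loads it.
; Once loaded, it reveals the effect and, if requested, async loads and plays the weapon type's sound.
; The actor destroys itself when particles finish or no tag matches.
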(event OnSystemFinished(ParticleSystem)
  (params (PSystem :type Particle%20System%20Component%20Object%20Reference))
  (Actor|DestroyActor))

(event Custom|SetTag
  (params (SurfaceTags :type Array%20of%20Names) (Size :type EImpactSize%20Enum :default "NewEnumerator0") (bMakeSound :type Boolean) (WeaponType :type EWeaponType%20Enum :default "NewEnumerator0"))
  (bind _particlesystem (Variables|Default|GetParticleSystem))
  (bind _impactsound (Variables|Default|GetImpactSound))
  (bind (_value _returnvalue) (Utilities|Map|Find _impactsound WeaponType))
  (bind _array_element (Utilities|Array|ForEachLoopwithBreak SurfaceTags :!label _label)
    (:LoopBody
      (if (.ReturnValue (Utilities|Map|Find (Variables|Default|GetSurfaceMap) _array_element))
        (Variables|Default|SetSurfaceTag _array_element)
        (goto _label Break)))
    (:Completed
      (if (Utilities|Name|NotEqual(Name) (Variables|Default|GetSurfaceTag) "None")
        (bind _object (Utilities|AsyncLoadAsset (Utilities|Array|Get(acopy) (Utilities|Struct|BreakSImpactPS (.Value (Utilities|Map|Find (Variables|Default|GetSurfaceMap) (Variables|Default|GetSurfaceTag)))) (Utilities|Select :Index Size :NewEnumerator0 0 :NewEnumerator1 1 :NewEnumerator2 2)))
          (:Completed
            (Effects|Components|ParticleSystem|SetTemplate _particlesystem (.AsParticle%20System (Utilities|Casting|CastToParticleSystem _object)))
            (Development|SetHiddeninGame _particlesystem false false)
            (if (and bMakeSound _returnvalue)
              (bind _object_2 (Utilities|AsyncLoadAsset _value)
                (:Completed
                  (Audio|PlaySoundatLocation (.AsSound%20Cue (Utilities|Casting|CastToSoundCue _object_2)) (Transformation|GetActorLocation) "0, 0, 0" 1.0 1.0 0.0 0 0 0))))))
        (else
          (Actor|DestroyActor))))))

(fn ConstructionScript)