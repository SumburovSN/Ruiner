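; BP_TracerActor is a cosmetic tracer for trace weapons that flies a particle effect forward in a straight line.
; SetParams stores speed and destroy time, async-loads the given particle system, then applies it, unhides it and starts the lifespan.
; Tick moves the actor along its forward vector without sweeping, only after loading completes, so the tracer performs no collision or hit logic.
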(event Custom|SetParams
  (params (TracerSpeed :type Float%20%28single-precision%29) (DestroyTime :type Float%20%28single-precision%29) (ParticleSystem :type Particle%20System%20Soft%20Object%20Reference))
  (Variables|Default|SetTracerSpeed TracerSpeed)
  (Variables|Default|SetDestroyTime DestroyTime)
  (bind _object (Utilities|AsyncLoadAsset ParticleSystem)
    (:Completed
      (Effects|Components|ParticleSystem|SetTemplate (Variables|Default|GetParticleSystem) (.AsParticle%20System (Utilities|Casting|CastToParticleSystem _object)))
      (Development|SetHiddeninGame (Variables|Default|GetParticleSystem) false false)
      (Variables|Default|SetbParamsSet true)
      (Actor|SetLifeSpan (Variables|Default|GetDestroyTime)))))

(event EventBeginPlay)

(event Collision|EventActorBeginOverlap
  (params (OtherActor :type Actor%20Object%20Reference)))

(event EventTick
  (params (DeltaSeconds :type Float%20%28single-precision%29))
  (if (Variables|Default|GetbParamsSet)
    (Transformation|AddActorWorldOffset (* (Transformation|GetActorForwardVector) (* DeltaSeconds (Variables|Default|GetTracerSpeed))))))

(fn ConstructionScript)