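; Trace-based ammo weapon that fires a hitscan line with simulated projectile travel time.
; On firing, it traces from the muzzle along the owner's forward vector, leaving debug drawing enabled.
; Only on a hit, it spawns a tracer, then waits distance divided by tracer speed.
; It then spawns an impact actor, fed surface tags from any hit static mesh, and a configurable damage actor at the hit point.
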(event EventBeginPlay
  (|CallParentFunction) ; This node is disabled and will not be called.\nDrag off pins to build functionality.
)

(event Collision|EventActorBeginOverlap
  (params (OtherActor :type Actor%20Object%20Reference)))

(event EventTick
  (params (DeltaSeconds :type Float%20%28single-precision%29)))

(event EventOnFired
  (bind _returnvalue (Components|GetOwner))
  (bind _skeletalmesh (Variables|Default|GetSkeletalMesh))
  (bind _tracerspeed (Variables|Default|GetTracerSpeed))
  (bind _returnvalue_2 (Transformation|GetSocketLocation _skeletalmesh "Muzzle"))
  (|CallParentFunction)
  (bind (_outhit _returnvalue_3) (Collision|LineTraceByChannel _returnvalue_2 (+ _returnvalue_2 (* (Transformation|GetActorForwardVector _returnvalue) (Variables|Default|GetTraceDistance))) "TraceTypeQuery1" false (Utilities|Array|MakeArray _returnvalue) "ForDuration"))
  (if _returnvalue_3
    (bind _returnvalue_4 (Game|SpawnActorfromClass "/Game/Ruiner/Core/Items/Equipables/Weapons/AmmoWeapons/TraceWeapons/BP_TracerActor.BP_TracerActor_C" (Math|Transform|MakeTransform _returnvalue_2 (Transformation|GetActorRotation (Components|GetOwner)) "1,1,1") "Undefined" self 0))
    (Default|SetParams _returnvalue_4 _tracerspeed (/ (.distance _outhit) _tracerspeed) (Variables|Default|GetTracerPS))
    (Utilities|FlowControl|Delay (/ (.distance _outhit) _tracerspeed))
    (bind _returnvalue_5 (Game|SpawnActorfromClass "/Game/Ruiner/Core/Items/Equipables/Weapons/AmmoWeapons/TraceWeapons/BP_ImpactActor.BP_ImpactActor_C" (Math|Transform|MakeTransform (.location _outhit) "0, 0, 0" "1,1,1") "Undefined" self 0))
    (Utilities|IsValid (Actor|GetComponentbyClass (.hitactor _outhit) "/Script/Engine.StaticMeshComponent")
      (:Is%20Valid
        (Default|SetTag _returnvalue_5 (Variables|/Script/Engine.ActorComponent|GetComponentTags (Actor|GetComponentbyClass (.hitactor _outhit) "/Script/Engine.StaticMeshComponent")) (Variables|Default|GetImpactSize) (Variables|Default|GetbMakeImpactSound) (Variables|Default|GetWeaponType)))
      (:Is%20Not%20Valid
        _))
    (Game|SpawnActorfromClass (Variables|Default|GetDamageActorClass) (Math|Transform|MakeTransform (.location _outhit) "0, 0, 0" "1,1,1") "Undefined" self 0)))

(fn ConstructionScript
  (|CallParentFunction))