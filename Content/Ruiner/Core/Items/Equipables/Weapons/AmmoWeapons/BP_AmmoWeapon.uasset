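; BP_AmmoWeapon is a weapon Blueprint that adds ammunition handling to its parent, filling CurAmmo to MaxAmmo on BeginPlay.
; Helper functions decrement ammo and check whether any remains.
; Magazine state comes from the single ammo count: the weapon counts as unloaded at each AmmoPerMag multiple unless Reloaded is set.
; The fire animation play rate scales WFire's length by ShotsPerSecond, so one playback matches one shot interval.
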(event EventBeginPlay
  (|CallParentFunction)
  (Variables|Default|SetCurAmmo (Variables|Default|GetMaxAmmo)))

(fn ConstructionScript
  (|CallParentFunction))

(fn UseAmmunition
  (Math|Integer|DecrementInt (Variables|Default|GetCurAmmo)))

(fn CheckLoaded
  (return (not (and (== (Math|Integer|%(Integer) (Variables|Default|GetCurAmmo) (Variables|Default|GetAmmoPerMag)) 0) (not (Variables|Default|GetbReloaded))))))

(fn CheckAmmunition
  (return (> (Variables|Default|GetCurAmmo) 0)))

(fn GetFireAnimationPlayRate
  (return (* (Variables|/Script/Engine.AnimSequenceBase|GetSequenceLength (Variables|Default|GetW_Fire)) (Variables|Default|GetShotsPerSecond))))