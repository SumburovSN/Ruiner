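; Base landmine actor that detonates when any pawn enters its trigger sphere.
; BeginPlay asynchronously loads the explosion sound and destruction particle assets and stores them for later.
; On overlap it spawns a configurable damage actor at the sphere, fires a radial force impulse, plays whichever effects have loaded, then destroys itself.
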(event OnComponentBeginOverlap(Sphere)
  (params (OverlappedComponent :type Primitive%20Component%20Object%20Reference) (OtherActor :type Actor%20Object%20Reference) (OtherComp :type Primitive%20Component%20Object%20Reference) (OtherBodyIndex :type Integer) (bFromSweep :type Boolean) (SweepResult :type Hit%20Result%20Structure%20%28by%20ref%29))
  (bind _explosioncueloaded (Variables|Default|GetExplosionCueLoaded))
  (bind _destroy_psloaded (Variables|Default|GetDestroy_PSLoaded))
  (bind _sphere (Variables|Default|GetSphere))
  (bind _returnvalue (Transformation|GetWorldLocation _sphere))
  (Utilities|Casting|CastToPawn OtherActor)
  (Game|SpawnActorfromClass (Variables|Default|GetDamageActorClass) (Math|Transform|MakeTransform (Transformation|GetWorldLocation (Variables|Default|GetSphere)) "0, 0, 0" "1,1,1") "Undefined" 0 0)
  (Class|RadialForceComponent|FireImpulse (Variables|Default|GetRadialForce))
  (Utilities|IsValid _explosioncueloaded
    (:Is%20Valid
      (Audio|SpawnSoundatLocation _explosioncueloaded _returnvalue "0, 0, 0" 1.0 1.0 0.0 0 0))
    (:Is%20Not%20Valid
      _))
  (Utilities|IsValid _destroy_psloaded
    (:Is%20Valid
      (Effects|SpawnEmitteratLocation _destroy_psloaded _returnvalue))
    (:Is%20Not%20Valid
      _))
  (Actor|DestroyActor))

(event EventBeginPlay
  (bind _object (Utilities|AsyncLoadAsset (Variables|Default|GetExplosionCue))
    (:then
      (bind _object_2 (Utilities|AsyncLoadAsset (Variables|Default|GetDestroy_PS))
        (:Completed
          (Variables|Default|SetDestroy_PSLoaded (.AsParticle%20System (Utilities|Casting|CastToParticleSystem _object_2))))))
    (:Completed
      (Variables|Default|SetExplosionCueLoaded (.AsSound%20Cue (Utilities|Casting|CastToSoundCue _object))))))

(fn ConstructionScript)