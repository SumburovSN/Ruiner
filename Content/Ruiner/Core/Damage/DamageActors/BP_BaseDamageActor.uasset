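; BP_BaseDamageActor is a base one-shot damage actor that acts once on BeginPlay and then destroys itself.
; It passes OverlapObjectTypes to ShapeOverlapObject, then applies DamageValue to each returned actor with itself as damage causer.
; ShapeOverlapObject is an empty stub here, so the base defines the query, damage and destroy sequence without any overlap shape.
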(event EventBeginPlay
  (bind _overlappedactors (CallFunction|ShapeOverlapObject (Variables|Default|GetOverlapObjectTypes)))
  (CallFunction|OnOverlapingActors _overlappedactors))

(fn ConstructionScript)

(fn ShapeOverlapObject
  (params (ObjectType :type Array%20of%20EObjectTypeQuery%20Enums :default "ObjectTypeQuery1"))
  (return 0))

(fn OnOverlapingActors
  (params (OverlappedActors :type Array%20of%20Actor%20Object%20References))
  (CallFunction|ApplyDamage OverlappedActors)
  (Actor|DestroyActor))

(fn ApplyDamage
  (params (inActors :type Array%20of%20Actor%20Object%20References))
  (for _array_element inActors
    (Game|Damage|ApplyDamage _array_element (Variables|Default|GetDamageValue) 0 self))
  (return))