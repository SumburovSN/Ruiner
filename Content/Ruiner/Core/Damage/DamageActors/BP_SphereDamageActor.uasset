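; Damage actor variant that uses a sphere as its area for finding targets.
; ShapeOverlapObject runs a sphere overlap at the actor's location with SphereRadius, filtered by the given object types, and returns the overlapped actors.
; An optional DrawDebug flag briefly draws the query sphere.
; The event graph is inactive and the file itself applies no damage, only supplying the overlap query.
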(event EventBeginPlay
  (|CallParentFunction) ; This node is disabled and will not be called.\nDrag off pins to build functionality.
)

(event Collision|EventActorBeginOverlap
  (params (OtherActor :type Actor%20Object%20Reference)))

(event EventTick
  (params (DeltaSeconds :type Float%20%28single-precision%29)))

(fn ConstructionScript
  (|CallParentFunction))

(fn ShapeOverlapObject
  (params (ObjectType :type Array%20of%20EObjectTypeQuery%20Enums :default "ObjectTypeQuery1"))
  (bind _returnvalue (Transformation|GetActorLocation))
  (bind _sphere_radius (Variables|Default|GetSphere%20Radius))
  (bind _outactors (Collision|SphereOverlapActors _returnvalue _sphere_radius ObjectType 0))
  (if (Variables|Default|GetbDrawDebug)
    (Rendering|Debug|DrawDebugSphere _returnvalue _sphere_radius 12 "(R=0.134695,G=0.049112,B=1.000000,A=1.000000)" 3.0 2.0))
  (return _outactors))