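; Capsule-shaped damage actor that supplies the overlap query for finding actors of a given object type.
; ShapeOverlapObject offsets the capsule center by its half height along the actor's up vector, putting the bottom at the actor's location, and returns the overlapping actors.
; An optional debug draw shows the capsule with the actor's rotation, while the overlap query itself takes no rotation.
; The event graph and construction script add no logic.
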(event EventBeginPlay
  (|CallParentFunction) ; This node is disabled and will not be called.\nDrag off pins to build functionality.
)

(event Collision|EventActorBeginOverlap
  (params (OtherActor :type Actor%20Object%20Reference)))

(event EventTick
  (params (DeltaSeconds :type Float%20%28single-precision%29)))

(fn ConstructionScript
  (|CallParentFunction))

(fn ShapeOverlapObject
  (params (ObjectType :type Array%20of%20EObjectTypeQuery%20Enums :default "ObjectTypeQuery1"))
  (bind _returnvalue (Transformation|GetActorLocation))
  (bind _returnvalue_2 (Transformation|GetActorUpVector))
  (bind _capsulehalfheight (Variables|Default|GetCapsuleHalfHeight))
  (bind _returnvalue_3 (* _returnvalue_2 _capsulehalfheight))
  (bind _returnvalue_4 (+ _returnvalue _returnvalue_3))
  (bind _outactors (Collision|CapsuleOverlapActors _returnvalue_4 (Variables|Default|GetCapsuleRadius) (Variables|Default|GetCapsuleHalfHeight) ObjectType 0))
  (if (Variables|Default|GetbDrawDebug)
    (Rendering|Debug|DrawDebugCapsule _returnvalue_4 (Variables|Default|GetCapsuleHalfHeight) (Variables|Default|GetCapsuleRadius) (Transformation|GetActorRotation) "(R=1.000000,G=0.061054,B=0.365273,A=1.000000)" 3.0 2.0))
  (return _outactors))