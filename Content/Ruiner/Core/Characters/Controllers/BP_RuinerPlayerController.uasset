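; Player controller for Ruiner, handling camera-relative movement, camera orbit and zoom, firing, reloading and inventory weapon switching.
; Tick traces under the cursor, turns the character toward it and fires while held.
; Tapping dash while moving dashes forward; holding it, or pressing while stationary, starts slow-motion target picking with a camera modifier.
; Picked points are range and line-of-sight checked, then dashed through on release, timeout or blocked sight to the first point.
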(event Custom|ActivateDashTargetPickingMode
  ;[1 1 1] PickingDashPoints Mode
  (Utilities|ActivatePicking))

(event Custom|DeactivateDashTargetPickingMode
  ;[1 1 1] PickingDashPoints Mode
  (Utilities|DeactivatePicking))

(event EventBeginPlay
  ;[1 1 1] Camera start
  (Variables|Default|SetRuinerPlayerCameraManager (.AsBP%20Ruiner%20Player%20Camera%20Manager (Utilities|Casting|CastToBP_RuinerPlayerCameraManager (Variables|Default|GetPlayerCameraManager))))
  (Variables|Default|SetRuinerHumanoidCharacter (.AsBP%20Ruiner%20Humanoid%20Character (Utilities|Casting|CastToBP_RuinerHumanoidCharacter (Pawn|GetControlledPawn))))
  (Actor|GetActorOfClass 0))

(event EventTick
  (params (DeltaSeconds :type Float%20%28single-precision%29))
  ;[1 1 1] Event Tick
  (Utilities|UpdateCursorHitResult)
  (Utilities|InterpCharacterRotation)
  (Utilities|EnsureCanDash)
  (Utilities|TrytoFire))

(event Input|ActionEvents|InputActionIncreaseCameraRadial
  (params (Key :type Key%20Structure :default "None"))
  ;[1 1 1] Camera Angle
  (:Pressed
    (Default|IncreaseRadialAngle (Variables|Default|GetRuinerPlayerCameraManager) 9e+01)))

(event Input|ActionEvents|InputActionDecreaseCameraRadial
  (params (Key :type Key%20Structure :default "None"))
  ;[1 1 1] Camera Angle
  (:Pressed
    (Default|IncreaseRadialAngle (Variables|Default|GetRuinerPlayerCameraManager) -9e+01)))

(event Input|ActionEvents|InputActionSelectSlot7
  (params (Key :type Key%20Structure :default "None"))
  ;[1 1 1] Select slot7
  (:Pressed
    (Default|EquipSlot (Variables|/Game/Ruiner/Core/Characters/Pawns/BP_RuinerHumanoidCharacter.BP_RuinerHumanoidCharacter_C|GetBP_InventoryComponent (Variables|Default|GetRuinerHumanoidCharacter)) "NewEnumerator6")))

(event Input|ActionEvents|InputActionSelectSlot1
  (params (Key :type Key%20Structure :default "None"))
  ;[1 1 1] Select Weapon('1..7' keys)
  (:Pressed
    (Default|EquipSlot (Variables|/Game/Ruiner/Core/Characters/Pawns/BP_RuinerHumanoidCharacter.BP_RuinerHumanoidCharacter_C|GetBP_InventoryComponent (Variables|Default|GetRuinerHumanoidCharacter)) "NewEnumerator0")))

(event Input|ActionEvents|InputActionSelectSlot2
  (params (Key :type Key%20Structure :default "None"))
  ;[1 1 1] Select Weapon('1..7' keys)
  (:Pressed
    (Default|EquipSlot (Variables|/Game/Ruiner/Core/Characters/Pawns/BP_RuinerHumanoidCharacter.BP_RuinerHumanoidCharacter_C|GetBP_InventoryComponent (Variables|Default|GetRuinerHumanoidCharacter)) "NewEnumerator1")))

(event Input|ActionEvents|InputActionSelectSlot1
  (params (Key :type Key%20Structure :default "None"))
  ;[1 1 1] Select slot1
  (:Pressed
    (Default|EquipSlot (Variables|/Game/Ruiner/Core/Characters/Pawns/BP_RuinerHumanoidCharacter.BP_RuinerHumanoidCharacter_C|GetBP_InventoryComponent (Variables|Default|GetRuinerHumanoidCharacter)) "NewEnumerator0")))

(event Input|ActionEvents|InputActionSelectSlot2
  (params (Key :type Key%20Structure :default "None"))
  ;[1 1 1] Select slot2
  (:Pressed
    (Default|EquipSlot (Variables|/Game/Ruiner/Core/Characters/Pawns/BP_RuinerHumanoidCharacter.BP_RuinerHumanoidCharacter_C|GetBP_InventoryComponent (Variables|Default|GetRuinerHumanoidCharacter)) "NewEnumerator1")))

(event Input|ActionEvents|InputActionSelectSlot3
  (params (Key :type Key%20Structure :default "None"))
  ;[1 1 1] Select slot3
  (:Pressed
    (Default|EquipSlot (Variables|/Game/Ruiner/Core/Characters/Pawns/BP_RuinerHumanoidCharacter.BP_RuinerHumanoidCharacter_C|GetBP_InventoryComponent (Variables|Default|GetRuinerHumanoidCharacter)) "NewEnumerator2")))

(event Input|ActionEvents|InputActionDashTargetPick
  (params (Key :type Key%20Structure :default "None"))
  ;[1 1 1] RMB - DashTargetPicking Mode
  (:Pressed
    (Utilities|DashTargetPick :!label _label))
  (:Released
    (goto _label execute2)))

(event Input|ActionEvents|InputActionSelectSlot4
  (params (Key :type Key%20Structure :default "None"))
  ;[1 1 1] Select Weapon('1..7' keys)
  (:Pressed
    (Default|EquipSlot (Variables|/Game/Ruiner/Core/Characters/Pawns/BP_RuinerHumanoidCharacter.BP_RuinerHumanoidCharacter_C|GetBP_InventoryComponent (Variables|Default|GetRuinerHumanoidCharacter)) "NewEnumerator3")))

(event Input|ActionEvents|InputActionSelectSlot5
  (params (Key :type Key%20Structure :default "None"))
  ;[1 1 1] Select Weapon('1..7' keys)
  (:Pressed
    (Default|EquipSlot (Variables|/Game/Ruiner/Core/Characters/Pawns/BP_RuinerHumanoidCharacter.BP_RuinerHumanoidCharacter_C|GetBP_InventoryComponent (Variables|Default|GetRuinerHumanoidCharacter)) "NewEnumerator4")))

(event Input|ActionEvents|InputActionSelectSlot6
  (params (Key :type Key%20Structure :default "None"))
  ;[1 1 1] Select Weapon('1..7' keys)
  (:Pressed
    (Default|EquipSlot (Variables|/Game/Ruiner/Core/Characters/Pawns/BP_RuinerHumanoidCharacter.BP_RuinerHumanoidCharacter_C|GetBP_InventoryComponent (Variables|Default|GetRuinerHumanoidCharacter)) "NewEnumerator5")))

(event Input|ActionEvents|InputActionSelectSlot7
  (params (Key :type Key%20Structure :default "None"))
  ;[1 1 1] Select Weapon('1..7' keys)
  (:Pressed
    (Default|EquipSlot (Variables|/Game/Ruiner/Core/Characters/Pawns/BP_RuinerHumanoidCharacter.BP_RuinerHumanoidCharacter_C|GetBP_InventoryComponent (Variables|Default|GetRuinerHumanoidCharacter)) "NewEnumerator6")))

(event Input|ActionEvents|InputActionSelectSlot4
  (params (Key :type Key%20Structure :default "None"))
  ;[1 1 1] Select slot4
  (:Pressed
    (Default|EquipSlot (Variables|/Game/Ruiner/Core/Characters/Pawns/BP_RuinerHumanoidCharacter.BP_RuinerHumanoidCharacter_C|GetBP_InventoryComponent (Variables|Default|GetRuinerHumanoidCharacter)) "NewEnumerator3")))

(event Input|ActionEvents|InputActionSelectSlot5
  (params (Key :type Key%20Structure :default "None"))
  ;[1 1 1] Select slot5
  (:Pressed
    (Default|EquipSlot (Variables|/Game/Ruiner/Core/Characters/Pawns/BP_RuinerHumanoidCharacter.BP_RuinerHumanoidCharacter_C|GetBP_InventoryComponent (Variables|Default|GetRuinerHumanoidCharacter)) "NewEnumerator4")))

(event Input|ActionEvents|InputActionSelectSlot6
  (params (Key :type Key%20Structure :default "None"))
  ;[1 1 1] Select slot6
  (:Pressed
    (Default|EquipSlot (Variables|/Game/Ruiner/Core/Characters/Pawns/BP_RuinerHumanoidCharacter.BP_RuinerHumanoidCharacter_C|GetBP_InventoryComponent (Variables|Default|GetRuinerHumanoidCharacter)) "NewEnumerator5")))

(event Input|ActionEvents|InputActionDashConfirm
  (params (Key :type Key%20Structure :default "None"))
  ;[1 1 1] LMB - DashConfirm
  (:Pressed
    (CallFunction|DashConfirm)))

(event Input|ActionEvents|InputActionFire
  (params (Key :type Key%20Structure :default "None"))
  ;[1 1 1] Fire (LMB)
  (:Pressed
    (if (not (Variables|Default|GetbPickingDashTargets))
      (Variables|Default|SetbFiring true)))
  (:Released
    (Variables|Default|SetbFiring false)))

(event Input|ActionEvents|InputActionSelectSlot3
  (params (Key :type Key%20Structure :default "None"))
  ;[1 1 1] Select Weapon('1..7' keys)
  (:Pressed
    (Default|EquipSlot (Variables|/Game/Ruiner/Core/Characters/Pawns/BP_RuinerHumanoidCharacter.BP_RuinerHumanoidCharacter_C|GetBP_InventoryComponent (Variables|Default|GetRuinerHumanoidCharacter)) "NewEnumerator2")))

(event Input|AxisEvents|InputAxisMoveForward
  (params (AxisValue :type Float%20%28single-precision%29))
  ;[1 1 1] Movement
  (Pawn|Input|AddMovementInput (Variables|Default|GetRuinerHumanoidCharacter) (Math|Vector|GetForwardVector (Math|Rotator|MakeRotator 0.0 0.0 (.yaw (Camera|GetCameraRotation (Variables|Default|GetRuinerPlayerCameraManager))))) AxisValue false))

(event Input|AxisEvents|InputAxisMoveRight
  (params (AxisValue :type Float%20%28single-precision%29))
  ;[1 1 1] Movement
  (Pawn|Input|AddMovementInput (Variables|Default|GetRuinerHumanoidCharacter) (Math|Vector|GetRightVector (Math|Rotator|MakeRotator 0.0 0.0 (.yaw (Camera|GetCameraRotation (Variables|Default|GetRuinerPlayerCameraManager))))) AxisValue false))

(event Input|KeyboardEvents|R
  (params (Key :type Key%20Structure :default "None"))
  ;[1 1 1] Reload ('R' key)
  (:Pressed
    (bind _currentitem (Default|GetCurrentItem (Variables|/Game/Ruiner/Core/Characters/Pawns/BP_RuinerHumanoidCharacter.BP_RuinerHumanoidCharacter_C|GetBP_InventoryComponent (Variables|Default|GetRuinerHumanoidCharacter))))
    (bind _asbp_base_weapon (Utilities|Casting|CastToBP_BaseWeapon _currentitem))
    (Default|Reload _asbp_base_weapon)))

(event Input|KeyboardEvents|Subtract
  (params (Key :type Key%20Structure :default "None"))
  ;[1 1 1] CameraDistance ('+/-' keys)
  (:Pressed
    (Default|IncreaseDistance (Variables|Default|GetRuinerPlayerCameraManager))))

(event Input|KeyboardEvents|Add
  (params (Key :type Key%20Structure :default "None"))
  ;[1 1 1] CameraDistance ('+/-' keys)
  (:Pressed
    (Default|ReduceDistance (Variables|Default|GetRuinerPlayerCameraManager))))

(event Input|KeyboardEvents|Tab
  (params (Key :type Key%20Structure :default "None"))
  ;[1 1 1] ChangeWeapon ('Tab' key) Iterative
  (:Pressed
    (CallFunction|ChangeWeaponsinCircle)))

(fn ConstructionScript)

(fn InitiateInstantDash
  (bind _ruinerhumanoidcharacter (Variables|Default|GetRuinerHumanoidCharacter))
  (bind _outpoint (Utilities|ValidateDashPoint (+ (Transformation|GetActorLocation _ruinerhumanoidcharacter) (* (Transformation|GetActorForwardVector _ruinerhumanoidcharacter) (Variables|Dash|GetInstantDashLength))))
    (:isValid
      (Default|TryInitiateDash _ruinerhumanoidcharacter (Utilities|Array|MakeArray _outpoint)))))

(fn TryInitiateMultiPointDash
  (bind _dashtargetlocations (Variables|Default|GetDashTargetLocations))
  (if (Utilities|Array|IsValidIndex (Variables|Default|GetDashTargetLocations))
    (Utilities|Array|Reverse _dashtargetlocations)
    (Default|TryInitiateDash (Variables|Default|GetRuinerHumanoidCharacter) _dashtargetlocations)
    (Utilities|Array|Clear (Variables|Default|GetDashTargetLocations))))

(fn ChangeWeaponsinCircle
  (bind _ruinerhumanoidcharacter (Variables|Default|GetRuinerHumanoidCharacter))
  (bind _bp_inventorycomponent (Variables|/Game/Ruiner/Core/Characters/Pawns/BP_RuinerHumanoidCharacter.BP_RuinerHumanoidCharacter_C|GetBP_InventoryComponent _ruinerhumanoidcharacter))
  (bind _keys (Utilities|Map|Keys (Variables|/Game/Ruiner/Core/Characters/Components/BP_InventoryComponent.BP_InventoryComponent_C|GetItems _bp_inventorycomponent)))
  (if (== (Utilities|Array|FindItem _keys (Variables|/Game/Ruiner/Core/Characters/Components/BP_InventoryComponent.BP_InventoryComponent_C|GetCurrentSlot _bp_inventorycomponent)) (Utilities|Array|LastIndex _keys))
    (Default|EquipSlot _bp_inventorycomponent (Utilities|Array|Get(acopy) _keys))
    (else
      (bind _result (Math|Integer|IncrementInt (Utilities|Array|FindItem _keys (Variables|/Game/Ruiner/Core/Characters/Components/BP_InventoryComponent.BP_InventoryComponent_C|GetCurrentSlot _bp_inventorycomponent)))
        (:%20%20
          (Default|EquipSlot _bp_inventorycomponent (Utilities|Array|Get(acopy) _keys _result)))))))

(fn DashConfirm
  (bind _cursorhitresult (Variables|Default|GetCursorHitResult))
  (bind _location (Collision|BreakHitResult _cursorhitresult))
  (if (and (Variables|Default|GetbPickingDashTargets) (< (Utilities|Array|Length (Variables|Default|GetDashTargetLocations)) (Variables|Dash|GetDashMaxPoints)))
    (bind _outpoint (Utilities|ValidateDashPoint (+ _location "0, 0,90.000000"))
      (:isValid
        (Utilities|Array|Add (Variables|Default|GetDashTargetLocations) _outpoint)
        (bind _returnvalue (Game|SpawnActorfromClass "/Game/Ruiner/Art/BP_TargetPoint.BP_TargetPoint_C" (Math|Transform|MakeTransform _location "-90.000000, 0, 0" "0.200000,0.200000,0.200000") "Undefined" 0 0))
        (Utilities|Array|Add (Variables|Default|GetDashPoints) _returnvalue)))))