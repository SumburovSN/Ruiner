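; Inventory component for Ruiner humanoid characters that holds items by slot and handles switching the equipped one.
; On BeginPlay it spawns the initial items, attaches them hidden to the owner's mesh at their bones, then equips the current slot.
; EquipSlot swaps visibility and equip state, flagging weapons as in use.
; Weapon reloads block slot changes for the reload time, and DestroyAllItems destroys every held item.
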(event Custom|Init
  (bind _returnvalue (Components|GetOwner))
  (for _array_element (Variables|Default|GetInitialItems)
    (bind _returnvalue_2 (Game|SpawnActorfromClass _array_element (Math|Transform|MakeTransform (Transformation|GetActorLocation _returnvalue) "0, 0, 0" "1,1,1") "Undefined" _returnvalue 0))
    (Transformation|AttachComponentToComponent _returnvalue_2 (Variables|/Script/Engine.Character|GetMesh (.AsBP%20Ruiner%20Humanoid%20Character (Utilities|Casting|CastToBP_RuinerHumanoidCharacter (Components|GetOwner)))) (Variables|/Game/Ruiner/Core/Items/Equipables/BP_BaseEquipable.BP_BaseEquipable_C|GetAttachBone _returnvalue_2) "KeepRelative" "KeepRelative" "KeepRelative" true)
    (Transformation|SetActorRelativeTransform _returnvalue_2 (Variables|/Game/Ruiner/Core/Items/Equipables/BP_BaseEquipable.BP_BaseEquipable_C|GetTransformRelative _returnvalue_2) false false)
    (Utilities|Map|Add (Variables|Default|GetItems) (Variables|/Game/Ruiner/Core/Items/Equipables/BP_BaseEquipable.BP_BaseEquipable_C|GetSetupSlot _returnvalue_2) _returnvalue_2)
    (Rendering|SetActorHiddenInGame _returnvalue_2 true)
    (Default|OnPickedUp _returnvalue_2 (.AsBP%20Ruiner%20Humanoid%20Character (Utilities|Casting|CastToBP_RuinerHumanoidCharacter (Components|GetOwner)))))
  (CallFunction|EquipSlot (Variables|Default|GetCurrentSlot)))

(event Custom|EquipSlot
  (params (Slot :type EEquipableSlot%20Enum :default "NewEnumerator0"))
  (if (Math|Boolean|ANDBoolean (.ReturnValue (Utilities|Map|Find (Variables|Default|GetItems) (Variables|Default|GetCurrentSlot))) (.ReturnValue (Utilities|Map|Find (Variables|Default|GetItems) Slot)) (Variables|Default|GetbCanChangeSlot))
    (Utilities|IsValid (Variables|Default|GetCurrentItem)
      (:Is%20Valid
        (bind _can_unequip (Default|CanUnequipItem (Variables|Default|GetCurrentItem)))
        (if _can_unequip
          (Default|OnUnequipped (Variables|Default|GetCurrentItem))
          (bind _asbp_base_weapon (Utilities|Casting|CastToBP_BaseWeapon (Variables|Default|GetCurrentItem))
            (:then
              (Variables|/Game/Ruiner/Core/Items/Equipables/Weapons/BP_BaseWeapon.BP_BaseWeapon_C|SetbInUse _asbp_base_weapon false))
            (:CastFailed
              _))
          (Rendering|SetActorHiddenInGame (Variables|Default|GetCurrentItem) true)
          (Variables|Default|SetCurrentSlot Slot :!label _label)
          (bind _output_get (Variables|Default|SetCurrentItem (.Value (Utilities|Map|Find (Variables|Default|GetItems) (Variables|Default|GetCurrentSlot)))))
          (Default|OnEquipped _output_get)
          (Rendering|SetActorHiddenInGame _output_get false)
          (bind _asbp_base_weapon_2 (Utilities|Casting|CastToBP_BaseWeapon (Variables|Default|GetCurrentItem)))
          (EventDispatchers|BindEventtoOnReload _asbp_base_weapon_2 (delegate Custom|OnWeaponReload))
          (EventDispatchers|BindEventtoOnReload _asbp_base_weapon_2 (EventDispatchers|CreateEvent (.AsBP%20Ruiner%20Humanoid%20Character (Utilities|Casting|CastToBP_RuinerHumanoidCharacter (Components|GetOwner))) :!event OnReloadWeapon))
          (Variables|/Game/Ruiner/Core/Items/Equipables/Weapons/BP_BaseWeapon.BP_BaseWeapon_C|SetbInUse _asbp_base_weapon_2 true)))
      (:Is%20Not%20Valid
        (goto _label)))))

(event Custom|DestroyAllItems
  (bind _items (Variables|Default|GetItems))
  (bind _keys (Utilities|Map|Keys _items))
  (for _array_element _keys
    (Utilities|IsValid (.Value (Utilities|Map|Find _items _array_element))
      (:Is%20Valid
        (Actor|DestroyActor (.Value (Utilities|Map|Find _items _array_element)))))))

(event Custom|OnWeaponReload
  (params (ReloadTime :type Float%20%28single-precision%29))
  (Variables|Default|SetbCanChangeSlot false)
  (Utilities|FlowControl|RetriggerableDelay ReloadTime)
  (Variables|Default|SetbCanChangeSlot true))

(event EventBeginPlay
  (CallFunction|Init))

(fn GetCurrentItem
  (return (Variables|Default|GetCurrentItem)))

(fn GetActiveSlot
  (return (Variables|Default|GetCurrentSlot)))