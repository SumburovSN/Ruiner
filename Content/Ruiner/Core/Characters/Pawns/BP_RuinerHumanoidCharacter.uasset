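; Humanoid character Blueprint for Ruiner that handles a charge-based, multi-point dash plus weapon fire and reload.
; TryInitiateDash spends a charge and stores target locations, which Tick traverses from the array's end using curve-driven, unswept lerps.
; Charges recharge one at a time outside dashes, and their count is debug-printed every tick.
; Firing uses the inventory's current weapon, while reload scales its montage to the duration and suspends hand IK.
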(event Custom|FireWeapon
  (bind _currentitem (Default|GetCurrentItem (Variables|Default|GetBP_InventoryComponent)))
  (bind _asbp_base_weapon (Utilities|Casting|CastToBP_BaseWeapon _currentitem))
  (Default|Fire _asbp_base_weapon))

(event Custom|OnReloadWeapon
  (params (ReloadDuration :type Float%20%28single-precision%29))
  (bind _currentitem (Default|GetCurrentItem (Variables|Default|GetBP_InventoryComponent)))
  (bind _asbp_base_weapon (Utilities|Casting|CastToBP_BaseWeapon _currentitem))
  (bind _asabp_mannequin (Utilities|Casting|CastToABP_Mannequin (Components|SkeletalMesh|GetAnimInstance (Variables|Character|GetMesh))))
  (Default|SetUpdateHandIK _asabp_mannequin false)
  (bind _returnvalue (Animation|PlayAnimMontage (Variables|/Game/Ruiner/Core/Items/Equipables/Weapons/BP_BaseWeapon.BP_BaseWeapon_C|GetC_Reload _asbp_base_weapon) (/ (Variables|/Script/Engine.AnimSequenceBase|GetSequenceLength (Variables|/Game/Ruiner/Core/Items/Equipables/Weapons/BP_BaseWeapon.BP_BaseWeapon_C|GetC_Reload _asbp_base_weapon)) ReloadDuration) "None"))
  (if (!= _returnvalue 0.0)
    (Utilities|FlowControl|RetriggerableDelay ReloadDuration)
    (Default|SetUpdateHandIK _asabp_mannequin true)))

(event EventBeginPlay
  (Variables|Default|SetDashCharges (Variables|Dash|GetMaxDashCharges)))

(event Collision|EventActorBeginOverlap
  (params (OtherActor :type Actor%20Object%20Reference)))

(event EventTick
  (params (DeltaSeconds :type Float%20%28single-precision%29))
  (Utilities|Dash)
  (Utilities|RechargeDash)
  (Development|PrintString (Utilities|String|Append (Utilities|String|ToString(Integer) (Variables|Default|GetDashCharges)) "/" (Utilities|String|ToString(Integer) (Variables|Dash|GetMaxDashCharges))) true true "(R=0.000000,G=0.660000,B=1.000000,A=1.000000)" (Utilities|Time|GetWorldDeltaSeconds)))

(fn ConstructionScript)

(fn TryInitiateDash
  (params (Locations :type Array%20of%20Vectors))
  (if (CallFunction|IsAbletoDash)
    (Utilities|MakePreDashLocationSnapshot)
    (Variables|Default|SetDashQueries Locations)
    (Math|Integer|DecrementInt (Variables|Default|GetDashCharges)
      (:%20%20
        (Variables|Default|SetDashChargeTimer 0.0)))))

(fn IsDashinProgress
  (return (Utilities|Array|IsValidIndex (Variables|Default|GetDashQueries))))

(fn IsAbletoDash
  (return (and (not (CallFunction|IsDashinProgress)) (> (Variables|Default|GetDashCharges) 0))))