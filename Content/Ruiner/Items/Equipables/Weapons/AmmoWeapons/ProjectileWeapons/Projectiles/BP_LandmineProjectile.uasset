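; Landmine projectile for an ammo weapon that scatters into child projectiles and deploys landmines.
; On split it spawns copies of its own class with a decremented split depth, launching each with randomized local-space horizontal velocity and a Z velocity drawn from the split speed range.
; When splitting ends it spawns the configured landmine class at its transform, then runs the parent's split-end logic.
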(event EventBeginPlay
  (|CallParentFunction) ; This node is disabled and will not be called.\nDrag off pins to build functionality.
)

(event Collision|EventActorBeginOverlap
  (params (OtherActor :type Actor%20Object%20Reference)))

(event EventTick
  (params (DeltaSeconds :type Float%20%28single-precision%29)))

(fn ConstructionScript
  (|CallParentFunction))

(fn OnSplit
  (bind _returnvalue (Math|Random|RandomUnitVector))
  (bind _minsplitvelocity (Variables|Default|GetMinSplitVelocity))
  (bind _maxsplitvelocity (Variables|Default|GetMaxSplitVelocity))
  (bind _returnvalue_2 (Math|Random|RandomFloatinRange _minsplitvelocity _maxsplitvelocity))
  (bind _returnvalue_3 (* _returnvalue _returnvalue_2))
  (for _index (range 0 (- (Variables|Default|GetSplitCount) 1))
    (bind _returnvalue_4 (Game|SpawnActorfromClass (Utilities|GetClass self) (Transformation|GetActorTransform) "Undefined" 0 (- (Variables|Default|GetSplitDepth) 1) 0))
    (Game|Components|ProjectileMovement|SetVelocityinLocalSpace (Variables|/Game/Ruiner/Core/Items/Equipables/Weapons/AmmoWeapons/ProjectileWeapons/Projectiles/BP_BaseProjectile.BP_BaseProjectile_C|GetProjectileMovement _returnvalue_4) (Math|Vector|MakeVector (.x _returnvalue_3) (.y _returnvalue_3) _returnvalue_2)))
  (return))

(fn OnSplitEnd
  (Game|SpawnActorfromClass (Variables|Default|GetLandmineClass) (Transformation|GetActorTransform) "Undefined" 0 0)
  (|CallParentFunction))